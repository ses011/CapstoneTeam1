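; BP_BasePlayer is a base player that moves forward automatically, with its world Y position locked.
; Every Tick it adds forward movement input, then resets its location to the fixed Y set on BeginPlay while keeping current X and Z.
; HandleSidewaysMovementFunction adds heavily scaled movement input along the actor's right vector from an axis value, but nothing in this file calls it.
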(event `self.ReceiveBeginPlay`
  (set `self.FixedY` -170.0))

(event `self.ReceiveTick`
  (params (DeltaSeconds :type "Float (single-precision)"))
  (bind (_returnvalue_x _returnvalue_y _returnvalue_z) (`KismetMathLibrary.BreakVector` (`self.K2_GetActorLocation`)))
  (`self.AddMovementInput` (`self.GetActorForwardVector`))
  (`self.K2_SetActorLocation` (`KismetMathLibrary.MakeVector` _returnvalue_x (`self.FixedY`) _returnvalue_z)))

(fn `HandleSidewaysMovementFunction`
  (params (MoveAxisValue :type "Float (double-precision)"))
  (`self.AddMovementInput` (`self.GetActorRightVector`) (* MoveAxisValue 1500.0)))

(fn `UserConstructionScript`)