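; PC_PlayerControllerTest is a test player controller that tracks left and right mouse button held states.
; On BeginPlay it shows the cursor, sets Game and UI input with the mouse locked, caches the possessed BP_Player and adds the IMC_PCT mapping context.
; Enhanced Input Started and Completed events set or clear LMBHeld and RMBHeld, printing debug strings.
; If the pawn cast fails, the mapping context is never added.
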(event `self.ReceiveBeginPlay`
  ;[1 1 1] Begin Play/Startup
  (`KismetSystemLibrary.PrintString` "Player controller ACTIVE")
  (set `self.bShowMouseCursor` true)
  (`WidgetBlueprintLibrary.SetInputMode_GameAndUIEx` self null "LockAlways" false)
  (bind _asbp_player (cast `/Game/Blueprints/Player/BP_Player` (`self.K2_GetPawn`)))
  (set `self.As BP Player` _asbp_player)
  (`EnhancedInputSubsystemInterface.AddMappingContext` (pcsubsystem `EnhancedInputLocalPlayerSubsystem` null) "/Game/Blueprints/Inputs/IMC_PCT.IMC_PCT" 0 (struct)))

(event `EnhancedInput|/Game/Blueprints/Inputs/IA_LMB_PCT`
  (params (ActionValue :type Boolean) (ElapsedSeconds :type "Float (double-precision)") (TriggeredSeconds :type "Float (double-precision)") (InputAction :type "InputAction Object Reference" :default "/Game/Blueprints/Inputs/IA_LMB_PCT.IA_LMB_PCT"))
  (:`Started`
    (`KismetSystemLibrary.PrintString` "LMB pressed" true true (struct :`G` 0.66 :`B` 1.0 :`A` 1.0) 0.5)
    (set `self.LMBHeld?` true))
  (:`Completed`
    (`KismetSystemLibrary.PrintString` "LMB released" true true (struct :`G` 0.66 :`B` 1.0 :`A` 1.0) 0.5)
    (set `self.LMBHeld?` false)))

(event `EnhancedInput|/Game/Blueprints/Inputs/IA_RMB_PCT`
  (params (ActionValue :type Boolean) (ElapsedSeconds :type "Float (double-precision)") (TriggeredSeconds :type "Float (double-precision)") (InputAction :type "InputAction Object Reference" :default "/Game/Blueprints/Inputs/IA_RMB_PCT.IA_RMB_PCT"))
  (:`Started`
    (`KismetSystemLibrary.PrintString` "RMB pressed" true true (struct :`G` 0.66 :`B` 1.0 :`A` 1.0) 0.5)
    (set `self.RMBHeld?` true))
  (:`Completed`
    (`KismetSystemLibrary.PrintString` "RMB released" true true (struct :`G` 0.66 :`B` 1.0 :`A` 1.0) 0.5)
    (set `self.RMBHeld?` false)))

(fn `UserConstructionScript`)