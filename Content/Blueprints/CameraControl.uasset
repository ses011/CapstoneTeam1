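; Serial-driven movement component that pushes its parent components forward and steers them with values read from a COM port.
; BeginPlay retries opening the port until it connects, then a self-calling ReadSerial loop polls lines on a short delay into Rotation.
; While Continue is set, Tick moves each parent along its horizontal forward vector with sweep and adds scaled Rotation to yaw, without delta-time scaling.
; EndPlay closes the connection.
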(event `ReadSerial`
  (`KismetSystemLibrary.Delay` 0.25)
  (bind (_bsuccess _returnvalue) (`SerialCom.Readln` (`self.Connection`)))
  (if _bsuccess
    (set `self.Rotation` (`KismetStringLibrary.Conv_StringToDouble` _returnvalue)))
  (`self.ReadSerial`))

(event `self.ReceiveBeginPlay`
  (set `self.Parents` (`self.GetParentComponents`))
  (`KismetSystemLibrary.Delay` 0.3 :!label _label)
  (bind (_bopened _returnvalue) (`SerialCom.OpenComPortWithFlowControl` (`self.PortNum`) 9600 false))
  (if _bopened
    (bind _output_get (set `self.Connection` _returnvalue))
    (`SerialCom.Flush` _output_get)
    (`KismetSystemLibrary.PrintString` "Connect port")
    (`self.ReadSerial`)
    (else
      (goto _label))))

(event `self.ReceiveEndPlay`
  (params (EndPlayReason :type "EEndPlayReason Enum" :default "Destroyed"))
  (`SerialCom.Close` (`self.Connection`)))

(event `self.ReceiveTick`
  (params (DeltaSeconds :type "Float (single-precision)"))
  (bind _speed (`self.Speed`))
  ;[1 1 1] Move Player forward ever tick (WORKING)
  (if (`self.continue`)
    (for _array_element (`self.Parents`)
      (`|ExecutionSequence`
        (:`then_0`
          (bind (_returnvalue_x _returnvalue_y _returnvalue_z) (`KismetMathLibrary.BreakVector` (`self.K2_GetComponentLocation` _array_element)))
          (bind (_returnvalue_x_2 _returnvalue_y_2) (`KismetMathLibrary.BreakVector` (`self.GetForwardVector` _array_element)))
          (`self.K2_SetWorldLocation` _array_element (`KismetMathLibrary.MakeVector` (+ _returnvalue_x (* _returnvalue_x_2 1.0 _speed)) (+ _returnvalue_y (* _returnvalue_y_2 1.0 _speed)) _returnvalue_z) true false))
        (:`then_1`
          (bind (_returnvalue_roll _returnvalue_pitch _returnvalue_yaw) (`KismetMathLibrary.BreakRotator` (`self.K2_GetComponentRotation` _array_element)))
          (`self.K2_SetWorldRotation` _array_element (`KismetMathLibrary.MakeRotator` _returnvalue_roll _returnvalue_pitch (+ (/ (`self.Rotation`) 50.0) _returnvalue_yaw)) false false))))))