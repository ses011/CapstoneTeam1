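; Player controller for the Rave game that routes sideways movement input to the possessed player pawn.
; On possess it adds the IMC_RaveGame Enhanced Input mapping context.
; The separate P1 and P2 move actions both cast the controlled pawn to BP_BasePlayer and call its sideways movement handler.
; Controller ID checks with debug prints for telling the players apart are disconnected and never run.
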(event `self.ReceivePossess`
  (params (PossessedPawn :type "Pawn Object Reference"))
  (bind _returnvalue (subsystem `EnhancedInputWorldSubsystem`))
  (if (`KismetSystemLibrary.IsValid` _returnvalue)
    (message `EnhancedInputSubsystemInterface.AddMappingContext` _returnvalue "/Game/Input/IMC_RaveGame.IMC_RaveGame" 0 (struct))))

(event `EnhancedInput|/Game/Input/IA_Move_P2`
  (params (ActionValue :type "Float (double-precision)") (ElapsedSeconds :type "Float (double-precision)") (TriggeredSeconds :type "Float (double-precision)") (InputAction :type "InputAction Object Reference" :default "/Game/Input/IA_Move_P2.IA_Move_P2"))
  (:`Triggered`
    (bind _asbp_base_player (cast `/Game/BP_BasePlayer` (`self.K2_GetPawn`)))
    (`/Game/BP_BasePlayer.HandleSidewaysMovementFunction` _asbp_base_player ActionValue)))

(event `EnhancedInput|/Game/Input/IA_Move_P1`
  (params (ActionValue :type "Float (double-precision)") (ElapsedSeconds :type "Float (double-precision)") (TriggeredSeconds :type "Float (double-precision)") (InputAction :type "InputAction Object Reference" :default "/Game/Input/IA_Move_P1.IA_Move_P1"))
  (:`Triggered`
    (bind _asbp_base_player (cast `/Game/BP_BasePlayer` (`self.K2_GetPawn`)))
    (`/Game/BP_BasePlayer.HandleSidewaysMovementFunction` _asbp_base_player ActionValue)))

(fn `UserConstructionScript`)